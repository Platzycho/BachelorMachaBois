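; Player controller for a rhythm game that turns key presses into lane hits.
; Eight input actions (A, W, S, D and the four directions) each cast the game mode to RythmGameMode and call HandleLaneInput with a fixed lane number.
; Only presses are handled, with hit logic left to the game mode.
; BeginPlay prints a debug string, and Tick and the construction script are empty.
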(event `self.ReceiveBeginPlay`
  (`KismetSystemLibrary.PrintString` "Oogie Boogie"))

(event `InputAction|Hit_A`
  (params (Key :type "Key Structure"))
  (:`Pressed`
    (bind _asrythm_game_mode (cast `RythmGameMode` (`GameplayStatics.GetGameMode`)))
    (`RythmGameMode.HandleLaneInput` _asrythm_game_mode 1)))

(event `InputAction|Hit_W`
  (params (Key :type "Key Structure"))
  (:`Pressed`
    (bind _asrythm_game_mode (cast `RythmGameMode` (`GameplayStatics.GetGameMode`)))
    (`RythmGameMode.HandleLaneInput` _asrythm_game_mode 2)))

(event `InputAction|Hit_S`
  (params (Key :type "Key Structure"))
  (:`Pressed`
    (bind _asrythm_game_mode (cast `RythmGameMode` (`GameplayStatics.GetGameMode`)))
    (`RythmGameMode.HandleLaneInput` _asrythm_game_mode 3)))

(event `InputAction|Hit_D`
  (params (Key :type "Key Structure"))
  (:`Pressed`
    (bind _asrythm_game_mode (cast `RythmGameMode` (`GameplayStatics.GetGameMode`)))
    (`RythmGameMode.HandleLaneInput` _asrythm_game_mode 4)))

(event `InputAction|Hit_Right`
  (params (Key :type "Key Structure"))
  (:`Pressed`
    (bind _asrythm_game_mode (cast `RythmGameMode` (`GameplayStatics.GetGameMode`)))
    (`RythmGameMode.HandleLaneInput` _asrythm_game_mode 5)))

(event `InputAction|Hit_Up`
  (params (Key :type "Key Structure"))
  (:`Pressed`
    (bind _asrythm_game_mode (cast `RythmGameMode` (`GameplayStatics.GetGameMode`)))
    (`RythmGameMode.HandleLaneInput` _asrythm_game_mode 6)))

(event `InputAction|Hit_Down`
  (params (Key :type "Key Structure"))
  (:`Pressed`
    (bind _asrythm_game_mode (cast `RythmGameMode` (`GameplayStatics.GetGameMode`)))
    (`RythmGameMode.HandleLaneInput` _asrythm_game_mode 7)))

(event `InputAction|Hit_Left`
  (params (Key :type "Key Structure"))
  (:`Pressed`
    (bind _asrythm_game_mode (cast `RythmGameMode` (`GameplayStatics.GetGameMode`)))
    (`RythmGameMode.HandleLaneInput` _asrythm_game_mode 8)))

(fn `UserConstructionScript`)