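; Player controller Blueprint for a rhythm game, holding leftover lane-input logic that is currently inactive.
; Eight node chains each cast the game mode to RythmGameMode and call HandleLaneInput with a fixed lane number.
; None of these chains is wired to an event, so they never run, and BeginPlay, Tick and the construction script are empty.
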(event `InputAction|Hit_A`
  (params (Key :type "Key Structure")))

(event `InputAction|Hit_W`
  (params (Key :type "Key Structure")))

(event `InputAction|Hit_S`
  (params (Key :type "Key Structure")))

(event `InputAction|Hit_D`
  (params (Key :type "Key Structure")))

(event `InputAction|Hit_Right`
  (params (Key :type "Key Structure")))

(event `InputAction|Hit_Up`
  (params (Key :type "Key Structure")))

(event `InputAction|Hit_Down`
  (params (Key :type "Key Structure")))

(event `InputAction|Hit_Left`
  (params (Key :type "Key Structure")))

(fn `UserConstructionScript`)